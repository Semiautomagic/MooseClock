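; BP_SpiinyCube is an actor that continuously spins its Cube component around the yaw axis.
; Each Tick increments a Rotation variable by one and applies it as the cube's world yaw, so spin speed depends on frame rate.
; At 360 the value resets to zero, skipping the rotation update for that frame.
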(event EventBeginPlay)

(event Collision|EventActorBeginOverlap
  (params (OtherActor :type Actor%20Object%20Reference)))

(event EventTick
  (params (DeltaSeconds :type Float%20%28single-precision%29))
  (Math|Float|IncrementFloat (Variables|Default|GetRotation)
    (:%20%20
      (if (>= (Variables|Default|GetRotation) 3.6e+02)
        (Variables|Default|SetRotation 0.0)
        (else
          (Transformation|SetWorldRotation (Variables|Default|GetCube) (Math|Rotator|MakeRotator 0.0 0.0 (Variables|Default|GetRotation)) false false))))))

(fn ConstructionScript)