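; BP_SettingKeeper is an actor in the main menu assets that holds and persists network, game time and keybind settings.
; On BeginPlay it loads the "Settings" slot, if present, into its variables through SG_Options.
; SetSaveData replaces those variables, and SaveData writes them to a newly created save object in that slot.
; Saving keeps only both player times from the game data, filling its other fields with constants.
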(event EventBeginPlay
  (CallFunction|LoadData))

(event Collision|EventActorBeginOverlap
  (params (OtherActor :type Actor%20Object%20Reference)))

(event EventTick
  (params (DeltaSeconds :type Float%20%28single-precision%29)))

(fn ConstructionScript)

(fn LoadData
  (bind _returnvalue (SaveGame|DoesSaveGameExist "Settings"))
  (if _returnvalue
    (bind _returnvalue_2 (SaveGame|LoadGamefromSlot "Settings"))
    (bind _output_get (Variables|Default|SetSaveSettings _returnvalue_2))
    (bind _assg_options (Utilities|Casting|CastToSG_Options _output_get))
    (Variables|Default|SetNetworkData (Variables|/Game/Maps/MainMenuAssets/SG_Options.SG_Options_C|GetNetwork _assg_options))
    (Variables|Default|SetGameData (Variables|/Game/Maps/MainMenuAssets/SG_Options.SG_Options_C|GetTimeStuff _assg_options))
    (Variables|Default|SetKeybindData (Variables|/Game/Maps/MainMenuAssets/SG_Options.SG_Options_C|GetKeys _assg_options))))

(fn SaveData
  (bind _gamedata (Variables|Default|GetGameData))
  (bind _returnvalue (SaveGame|CreateSaveGameObject "/Game/Maps/MainMenuAssets/SG_Options.SG_Options_C"))
  (bind _output_get (Variables|Default|SetSaveSettings _returnvalue))
  (bind _assg_options (Utilities|Casting|CastToSG_Options _output_get))
  (Variables|/Game/Maps/MainMenuAssets/SG_Options.SG_Options_C|SetNetwork _assg_options (Variables|Default|GetNetworkData))
  (Variables|/Game/Maps/MainMenuAssets/SG_Options.SG_Options_C|SetTimeStuff _assg_options (Utilities|Struct|MakeS_GameStruct (.p1time _gamedata) (.p2time _gamedata) 0 0 1))
  (Variables|/Game/Maps/MainMenuAssets/SG_Options.SG_Options_C|SetKeys _assg_options (Variables|Default|GetKeybindData))
  (bind _returnvalue_2 (SaveGame|SaveGametoSlot (Variables|Default|GetSaveSettings) "Settings"))
  (return _returnvalue_2))

(fn SetSaveData
  (params (Game :type S%20Game%20Struct%20Structure) (Network :type S%20Network%20Struct%20Structure) (Keys :type S%20Keybinds%20Structure))
  (Variables|Default|SetGameData Game)
  (Variables|Default|SetNetworkData Network)
  (Variables|Default|SetKeybindData Keys))