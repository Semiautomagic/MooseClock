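; BP_TestPawn is a test pawn that relays gamepad button presses to the GM_Menu game mode.
; On BeginPlay it casts the current game mode to GM_Menu and caches the reference.
; Input actions for the face buttons, D-pad, shoulders and stick clicks each pass their pressed Key to the game mode's CallButtonPressed, leaving all response logic to GM_Menu.
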(event EventBeginPlay
  (bind _asgm_menu (Utilities|Casting|CastToGM_Menu (Game|GetGameMode)))
  (Variables|Default|SetGameMode _asgm_menu))

(event Input|ActionEvents|InputActionGamepadX
  (params (Key :type Key%20Structure :default "None"))
  ;[1 1 1] Face Buttons
  (:Pressed
    (Default|CallButtonPressed (Variables|Default|GetGameMode) Key)))

(event Input|ActionEvents|InputActionGamepadA
  (params (Key :type Key%20Structure :default "None"))
  ;[1 1 1] Face Buttons
  (:Pressed
    (Default|CallButtonPressed (Variables|Default|GetGameMode) Key)))

(event Input|ActionEvents|InputActionStickButtonLeft
  (params (Key :type Key%20Structure :default "None"))
  ;[1 1 1] Stick Buttons
  (:Pressed
    (Default|CallButtonPressed (Variables|Default|GetGameMode) Key)))

(event Input|ActionEvents|InputActionStickButtonRight
  (params (Key :type Key%20Structure :default "None"))
  ;[1 1 1] Stick Buttons
  (:Pressed
    (Default|CallButtonPressed (Variables|Default|GetGameMode) Key)))

(event Input|ActionEvents|InputActionGamepadY
  (params (Key :type Key%20Structure :default "None"))
  ;[1 1 1] Face Buttons
  (:Pressed
    (Default|CallButtonPressed (Variables|Default|GetGameMode) Key)))

(event Input|ActionEvents|InputActionGamepadB
  (params (Key :type Key%20Structure :default "None"))
  ;[1 1 1] Face Buttons
  (:Pressed
    (Default|CallButtonPressed (Variables|Default|GetGameMode) Key)))

(event Input|ActionEvents|InputActionShoulderLeft
  (params (Key :type Key%20Structure :default "None"))
  ;[1 1 1] Shoulders
  (:Pressed
    (Default|CallButtonPressed (Variables|Default|GetGameMode) Key)))

(event Input|ActionEvents|InputActionShoulderRight
  (params (Key :type Key%20Structure :default "None"))
  ;[1 1 1] Shoulders
  (:Pressed
    (Default|CallButtonPressed (Variables|Default|GetGameMode) Key)))

(event Input|ActionEvents|InputActionDpadUp
  (params (Key :type Key%20Structure :default "None"))
  ;[1 1 1] Dpad
  (:Pressed
    (Default|CallButtonPressed (Variables|Default|GetGameMode) Key)))

(event Input|ActionEvents|InputActionDpadDn
  (params (Key :type Key%20Structure :default "None"))
  ;[1 1 1] Dpad
  (:Pressed
    (Default|CallButtonPressed (Variables|Default|GetGameMode) Key)))

(event Input|ActionEvents|InputActionDpadLeft
  (params (Key :type Key%20Structure :default "None"))
  ;[1 1 1] Dpad
  (:Pressed
    (Default|CallButtonPressed (Variables|Default|GetGameMode) Key)))

(event Input|ActionEvents|InputActionDpadRight
  (params (Key :type Key%20Structure :default "None"))
  ;[1 1 1] Dpad
  (:Pressed
    (Default|CallButtonPressed (Variables|Default|GetGameMode) Key)))

(fn ConstructionScript)